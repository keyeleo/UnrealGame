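; Ball Blueprint that moves its static mesh using a spline and a timeline, starting at BeginPlay.
; Each timeline update scales the track value by spline length to sample local-space location and rotation along the spline.
; The mesh's world position is set to StaticMeshComponent's current world location plus that local point, with the sampled rotation yawed a quarter turn.
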(event EventBeginPlay
  (bind _spline (Variables|Default|GetSpline))
  (bind _newtrack_0 (Timeline|Timeline_0 Play)
    (:Update
      (Transformation|SetWorldLocationAndRotation (Variables|Default|GetStaticMesh) (+ (Transformation|GetWorldLocation (Variables|Debug|GetStaticMeshComponent)) (Spline|GetLocationatDistanceAlongSpline _spline (* _newtrack_0 (Spline|GetSplineLength _spline)) "Local")) (Math|Rotator|MakeRotator (.Roll (Math|Rotator|BreakRotator (Spline|GetRotationatDistanceAlongSpline _spline (* _newtrack_0 (Spline|GetSplineLength _spline)) "Local"))) (.Pitch (Math|Rotator|BreakRotator (Spline|GetRotationatDistanceAlongSpline _spline (* _newtrack_0 (Spline|GetSplineLength _spline)) "Local"))) (+ (.Yaw (Math|Rotator|BreakRotator (Spline|GetRotationatDistanceAlongSpline _spline (* _newtrack_0 (Spline|GetSplineLength _spline)) "Local"))) 9e+01)) false false))))

(event Collision|EventActorBeginOverlap
  (params (OtherActor :type Actor%20Object%20Reference)))

(event EventTick
  (params (DeltaSeconds :type Float%20%28single-precision%29)))

(fn ConstructionScript)